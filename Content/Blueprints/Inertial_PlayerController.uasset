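; Player controller that lets the player switch possession between InertialCharacter pawns with the Possess input.
; On press, it scans all InertialCharacters for others within a short range and in the front hemisphere of the controlled pawn.
; It picks the lowest product of distance and facing angle, favoring close, centered candidates.
; SetInertialCharacter possesses that pawn, moves the view target to it, enables its tick and disables the previous pawn's tick.
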(event EventBeginPlay)

(event EventTick
  (params (DeltaSeconds :type Float%20%28single-precision%29)))

(event Input|ActionEvents|InputActionPossess
  (params (Key :type Key%20Structure :default "None"))
  (bind _returnvalue (Pawn|GetControlledPawn))
  (:Pressed
    (Variables|Default|SetDistanceDotAngle 1e+05)
    (Variables|Default|SetNearest%20Character 0)
    (Utilities|String|LogString "Input Possess")
    (bind _outactors (Actor|GetAllActorsOfClass "/Script/Inertial_Antics.InertialCharacter"))
    (for (_array_element _array_index) _outactors
      (if (not (== _returnvalue _array_element))
        (if (and (< (Math|Vector|VectorLength (- (Transformation|GetActorLocation _array_element) (Transformation|GetActorLocation _returnvalue))) 3e+02) (< (Class|KismetMathLibrary|DegAcos (Math|Vector|DotProduct (Math|Vector|Normalize (- (Transformation|GetActorLocation _array_element) (Transformation|GetActorLocation _returnvalue))) (Transformation|GetActorForwardVector _returnvalue))) 9e+01))
          (Utilities|String|LogString (Utilities|String|Append "possess " (Utilities|String|ToString(Integer) _array_index)) :!label _label)
          (if (< (* (Math|Vector|VectorLength (- (Transformation|GetActorLocation _array_element) (Transformation|GetActorLocation _returnvalue))) (Class|KismetMathLibrary|DegAcos (Math|Vector|DotProduct (Math|Vector|Normalize (- (Transformation|GetActorLocation _array_element) (Transformation|GetActorLocation _returnvalue))) (Transformation|GetActorForwardVector _returnvalue)))) (Variables|Default|GetDistanceDotAngle))
            (Variables|Default|SetDistanceDotAngle (* (Math|Vector|VectorLength (- (Transformation|GetActorLocation _array_element) (Transformation|GetActorLocation _returnvalue))) (Class|KismetMathLibrary|DegAcos (Math|Vector|DotProduct (Math|Vector|Normalize (- (Transformation|GetActorLocation _array_element) (Transformation|GetActorLocation _returnvalue))) (Transformation|GetActorForwardVector _returnvalue)))))
            (Variables|Default|SetNearest%20Character _array_element)
            (goto _label)))))
    (Utilities|IsValid (Variables|Default|GetNearest%20Character)
      (:Is%20Valid
        (CallFunction|SetInertialCharacter (Variables|Default|GetNearest%20Character))))))

(fn ConstructionScript)

(fn SetInertialCharacter
  (params (NewPawn :type Pawn%20Object%20Reference))
  (bind _output_get (Variables|Default|SetPreviousCharacter (Pawn|GetControlledPawn)))
  (Pawn|Possess NewPawn)
  (Game|Player|SetViewTargetwithBlend NewPawn 0.0 "VTBlend_Linear" 0.0 false)
  (Actor|Tick|SetActorTickEnabled NewPawn true)
  (Utilities|IsValid _output_get
    (:Is%20Valid
      (Actor|Tick|SetActorTickEnabled _output_get))))
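; Valve actor that the player can destroy while standing in its box trigger.
; Pawn overlap shows a SpecialAct_Not widget, swaps the mesh to a highlight material and arms CanDestroy; leaving removes the widgets, restores the material and disarms it.
; A box hit by a pawn also adds the widget.
; DetroyValve, not called within this file, destroys the armed valve and spawns Spark_BP at its location.
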(event OnComponentHit(Box)
  (params (HitComponent :type Primitive%20Component%20Object%20Reference) (OtherActor :type Actor%20Object%20Reference) (OtherComp :type Primitive%20Component%20Object%20Reference) (NormalImpulse :type Vector :default "0, 0, 0") (Hit :type Hit%20Result%20Structure%20%28by%20ref%29))
  (Utilities|Casting|CastToPawn OtherActor)
  (bind _returnvalue (UserInterface|CreateWidget "/Game/Scenes/SpecialAct_Not.SpecialAct_Not_C"))
  (UserInterface|Viewport|AddtoViewport _returnvalue 5))

(event OnComponentBeginOverlap(Box)
  (params (OverlappedComponent :type Primitive%20Component%20Object%20Reference) (OtherActor :type Actor%20Object%20Reference) (OtherComp :type Primitive%20Component%20Object%20Reference) (OtherBodyIndex :type Integer) (bFromSweep :type Boolean) (SweepResult :type Hit%20Result%20Structure%20%28by%20ref%29))
  (Utilities|Casting|CastToPawn OtherActor)
  (bind _returnvalue (UserInterface|CreateWidget "/Game/Scenes/SpecialAct_Not.SpecialAct_Not_C"))
  (UserInterface|Viewport|AddtoViewport _returnvalue 5)
  (Rendering|Material|SetMaterial (Variables|Default|GetStaticMesh) 0 "/Game/Models/hightvalve.hightvalve")
  (Variables|Default|SetcanDestroy true))

(event OnComponentEndOverlap(Box)
  (params (OverlappedComponent :type Primitive%20Component%20Object%20Reference) (OtherActor :type Actor%20Object%20Reference) (OtherComp :type Primitive%20Component%20Object%20Reference) (OtherBodyIndex :type Integer))
  (Utilities|Casting|CastToPawn OtherActor)
  (bind _foundwidgets (Widget|GetAllWidgetsOfClass "/Game/Scenes/SpecialAct_Not.SpecialAct_Not_C" true))
  (Widget|RemovefromParent _foundwidgets)
  (Rendering|Material|SetMaterial (Variables|Default|GetStaticMesh) 0 "/Game/Models/valve_mat.valve_mat")
  (Variables|Default|SetcanDestroy false))

(event EventBeginPlay)

(event Collision|EventActorBeginOverlap
  (params (OtherActor :type Actor%20Object%20Reference)))

(event EventTick
  (params (DeltaSeconds :type Float%20%28single-precision%29)))

(fn ConstructionScript)

(fn Highlight)

(fn DetroyValve
  (if (Variables|Default|GetcanDestroy)
    (Actor|DestroyActor)
    (Game|SpawnActorfromClass "/Game/Blueprints/Spark_BP.Spark_BP_C" (Math|Transform|MakeTransform (Transformation|GetActorLocation)) "Undefined" 0 0)))
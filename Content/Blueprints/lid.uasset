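; A lid actor that the player slides back and forth with the MoveX input axis.
; Each axis event negates the input, scales it by Speed and offsets the actor along its forward vector without sweeping.
; MoveDIstance accumulates the travel, and any step that would leave the range from just above zero to MaxMoveDistance is skipped rather than clamped.
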(event EventBeginPlay)

(event Collision|EventActorBeginOverlap
  (params (OtherActor :type Actor%20Object%20Reference)))

(event EventTick
  (params (DeltaSeconds :type Float%20%28single-precision%29)))

(event Input|AxisEvents|InputAxisMoveX
  (params (AxisValue :type Float%20%28single-precision%29))
  (bind _returnvalue (* AxisValue -1.0))
  (bind _speed (Variables|Default|GetSpeed))
  (bind _returnvalue_2 (* _returnvalue _speed))
  (if (<= (+ (Variables|Default|GetMoveDIstance) _returnvalue_2) (Variables|Default|GetMaxMoveDistance))
    (if (> (+ (Variables|Default|GetMoveDIstance) _returnvalue_2) 0.0)
      (Transformation|SetActorLocation (+ (Transformation|GetActorLocation) (* (Transformation|GetActorForwardVector) _returnvalue_2)) false false)
      (Variables|Default|SetMoveDIstance (+ (Variables|Default|GetMoveDIstance) _returnvalue_2)))))

(fn ConstructionScript)
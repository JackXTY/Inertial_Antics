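; Player ball pawn that walks, jumps by charged physics impulse with a predicted arc preview, and highlights the pawn in front via custom depth.
; On the ground it moves kinematically with swept offsets and manual falling; jumps switch on physics until a slow-speed ground trace lands it.
; Holding the mouse draws the arc with spline meshes, and release launches.
; Stopping control waits for landing, then disables tick and enables physics.
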(event EventBeginPlay)

(event Collision|EventActorBeginOverlap
  (params (OtherActor :type Actor%20Object%20Reference)))

(event EventTick
  (params (DeltaSeconds :type Float%20%28single-precision%29))
  (if (Variables|Default|GetStopingPlayer)
    (CallFunction|CheckGround DeltaSeconds)
    (Class|InertialPawn|StopPlayerControl)
    (else
      (|CallParentFunction DeltaSeconds)
      (CallFunction|TurnCamera DeltaSeconds)
      (Utilities|FlowControl|Sequence
        (:then_0
          (if (Variables|Default|GetOnGround)
            (CallFunction|Walk DeltaSeconds)
            (CallFunction|AfterWalk DeltaSeconds)
            (else
              (CallFunction|CheckGround DeltaSeconds))))
        (:then_1
          (bind _asinertial_player_controller (Utilities|Casting|CastToInertial_PlayerController (Game|GetPlayerController 0)))
          (bind _result (Default|FindPawninFront _asinertial_player_controller))
          (Utilities|IsValid _result
            (:Is%20Valid
              (Variables|Default|SethighlighMeshes (Actor|GetComponentsByClass _result "/Script/Engine.StaticMeshComponent"))
              (for _array_element (Actor|GetComponentsByClass _result "/Script/Engine.StaticMeshComponent")
                (Rendering|SetRenderCustomDepth _array_element true)))
            (:Is%20Not%20Valid
              (for _array_element_2 (Variables|Default|GethighlighMeshes)
                (Rendering|SetRenderCustomDepth _array_element_2 false))
              (Utilities|Array|Clear (Variables|Default|GethighlighMeshes)))))))))

(event EventOnMouseRelease
  (params (val :type Float%20%28single-precision%29))
  (if (Variables|Default|GetOnGround)
    (CallFunction|Jump val)
    (Variables|Default|SetOnGround false)
    (Variables|Default|SetjumpTime 0.0)
    (for _array_element (Variables|Default|GetSplineMeshes)
      (Rendering|ToggleVisibility _array_element false))))

(event EventOnMousePressing
  (params (val :type Float%20%28single-precision%29))
  (if (Variables|Default|GetOnGround)
    (CallFunction|DrawParabola val)))

(event EventStopPlayerControl
  (if (Variables|Default|GetOnGround)
    (Actor|Tick|SetActorTickEnabled false)
    (Variables|Default|SetStopingPlayer false)
    (Physics|SetSimulatePhysics (Variables|Default|GetSphere) true)
    (else
      (Variables|Default|SetStopingPlayer true))))

(event EventStartPlayerControl
  (Variables|Default|SetStopingPlayer false)
  (Physics|SetSimulatePhysics (Variables|Default|GetSphere) false))

(fn ConstructionScript)

(fn Walk
  (params (time :type Float%20%28double-precision%29))
  (bind _returnvalue (Class|InertialPawn|GetWalkDirection))
  (if (> (Math|Vector|VectorLength _returnvalue) 0.5)
    (if (Class|SceneComponent|IsAnySimulatingPhysics (Variables|Default|GetSphere))
      (Physics|SetSimulatePhysics (Variables|Default|GetSphere) false)
      (Development|PrintString "Still simulating"))
    (Transformation|SetActorLocation (+ (* _returnvalue (* time (Variables|Default|GetwalkPower))) (Transformation|GetActorLocation)) true false)))

(fn TurnCamera
  (params (Time :type Float%20%28double-precision%29))
  (bind _camera (Variables|Default|GetCamera))
  (bind _cameradistance (Variables|Default|GetcameraDistance))
  (bind _returnvalue (Transformation|GetRelativeTransform _camera))
  (bind _returnvalue_2 (* _cameradistance -1.0))
  (bind _rotation (Math|Transform|BreakTransform _returnvalue))
  (bind (_roll _pitch _yaw) (Math|Rotator|BreakRotator _rotation))
  (Transformation|SetRelativeRotation (Variables|Default|GetCamera) (Math|Rotator|MakeRotator _roll (Math|Float|Clamp(Float) (+ (* (* (Variables|Default|GetdeltaMouseY) Time) (Variables|Default|GetcameraRotationSpeed)) _pitch) (Variables|Default|GetcameraMinAngle) (Variables|Default|GetcameraMaxAngle)) _yaw) false false)
  (Variables|Default|SetdeltaMouseY 0.0)
  (Variables|/Script/Engine.SpringArmComponent|SetSocketOffset (Variables|Default|GetSpringArm) (Math|Vector|MakeVector (* (Math|Trig|Cos(Degrees) (Math|Float|Clamp(Float) (+ (* (* (Variables|Default|GetdeltaMouseY) Time) (Variables|Default|GetcameraRotationSpeed)) _pitch) (Variables|Default|GetcameraMinAngle) (Variables|Default|GetcameraMaxAngle))) _returnvalue_2) 0.0 (* _returnvalue_2 (Math|Trig|Sin(Degrees) (Math|Float|Clamp(Float) (+ (* (* (Variables|Default|GetdeltaMouseY) Time) (Variables|Default|GetcameraRotationSpeed)) _pitch) (Variables|Default|GetcameraMinAngle) (Variables|Default|GetcameraMaxAngle)))))))

(fn Jump
  (params (jump :type Float%20%28double-precision%29))
  (Physics|SetSimulatePhysics (Variables|Default|GetSphere) true)
  (Class|PrimitiveComponent|SetMassOverrideinKg (Variables|Default|GetSphere) "None" (Variables|Default|GetpawnMass) true)
  (Physics|AddImpulse (Variables|Default|GetSphere) (* (* jump (Variables|Default|GetjumpPower)) (Math|Vector|GetRightVector (Variables|Default|GetArrowMesh))) "None" false))

(fn CheckGround
  (params (Time :type Float%20%28double-precision%29))
  (if (> (Variables|Default|GetjumpTime) 1.0)
    (if (< (Math|Vector|VectorLength (Transformation|GetComponentVelocity (Variables|Default|GetSphere))) 1e+01)
      (bind _touchbottom (CallFunction|CheckifTouchBottom))
      (if _touchbottom
        (Variables|Default|SetOnGround true)
        (Physics|SetSimulatePhysics (Variables|Default|GetSphere) false)
        (Transformation|SetActorLocation (+ (Transformation|GetActorLocation) "0,0,0.100000") false false)))
    (else
      (Variables|Default|SetjumpTime (+ Time (Variables|Default|GetjumpTime))))))

(fn DrawParabola
  (params (val :type Float%20%28double-precision%29))
  (bind _spline (Variables|Default|GetSpline))
  (bind _splinemeshes (Variables|Default|GetSplineMeshes))
  (bind _outpathpositions (Class|GameplayStatics|BlueprintPredictProjectilePathbyTraceChannel (Transformation|GetActorLocation) (* (Math|Vector|GetRightVector (Variables|Default|GetArrowMesh)) (* val (* (/ (Variables|Default|GetjumpPower) (Variables|Default|GetpawnMass)) 1.0))) false 0.0 "ECC_WorldDynamic" false 0 "None" 0.0 12.0))
  (Utilities|String|LogString (Utilities|String|Append "path length: " (Utilities|String|ToString(Integer) (Utilities|Array|Length _outpathpositions))))
  (Spline|SetSplinePoints (Variables|Default|GetSpline) _outpathpositions "World" true)
  (if (!= (Utilities|Array|Length _outpathpositions) (Utilities|Array|Length (Variables|Default|GetSplineMeshes)))
    (for _array_element _splinemeshes
      (Components|DestroyComponent _array_element))
    (Utilities|Array|Clear _splinemeshes)
    (for _index (range 1 (Spline|GetNumberOfSplinePoints (Variables|Default|GetSpline)))
      (bind _returnvalue (AddComponent|AddSplineMeshComponent true))
      (Utilities|Array|Add (Variables|Default|GetSplineMeshes) _returnvalue)))
  (for (_array_element_2 _array_index) (Variables|Default|GetSplineMeshes)
    (SplineMesh|SetStartandEnd _array_element_2 (.Location (Spline|GetLocationandTangentatSplinePoint _spline _array_index "World")) (.Tangent (Spline|GetLocationandTangentatSplinePoint _spline _array_index "World")) (.Location (Spline|GetLocationandTangentatSplinePoint _spline (+ _array_index 1) "World")) (.Tangent (Spline|GetLocationandTangentatSplinePoint _spline (+ _array_index 1) "World")) true :!class /Script/Engine.SplineMeshComponent)
    (if (not (Variables|/Script/Engine.SceneComponent|GetbVisible _array_element_2))
      (Rendering|ToggleVisibility _array_element_2 false))))

(fn CheckifTouchBottom
  (bind _returnvalue (Transformation|GetActorLocation))
  (bind _returnvalue_2 (Collision|LineTraceByChannel _returnvalue (+ _returnvalue (Math|Vector|MakeVector 0.0 0.0 (* (+ (Components|Sphere|GetScaledSphereRadius (Variables|Default|GetSphere)) 1.0) -1.0))) "TraceTypeQuery1" false 0 "None"))
  (return _returnvalue_2))

(fn AfterWalk
  (params (Time :type Float%20%28double-precision%29))
  (bind _touchbottom (CallFunction|CheckifTouchBottom))
  (if _touchbottom
    (Variables|Default|SetFallingSpeed 0.0)
    (else
      (bind _output_get (Variables|Default|SetFallingSpeed (+ (* Time 5e+02) (Variables|Default|GetFallingSpeed))))
      (bind _returnvalue (Transformation|SetActorLocation (- (Transformation|GetActorLocation) (Math|Vector|MakeVector 0.0 0.0 (* Time _output_get))) true false))
      (if (not _returnvalue)
        (Variables|Default|SetFallingSpeed 0.0)))))
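; Test pawn that rotates itself directly by transform, with no inertia.
; The MoveX axis event adds a fixed roll step on every call, ignoring the axis value and teleporting physics.
; An unconnected branch holds older or unused logic that would slide the pawn along its forward vector by the inverted, speed-scaled axis value, keeping the tracked distance within a set range.
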(event EventBeginPlay)

(event Collision|EventActorBeginOverlap
  (params (OtherActor :type Actor%20Object%20Reference)))

(event EventTick
  (params (DeltaSeconds :type Float%20%28single-precision%29)))

(event Input|AxisEvents|InputAxisMoveX
  (params (AxisValue :type Float%20%28single-precision%29))
  (bind _returnvalue (Transformation|GetActorRotation))
  (bind (_roll _pitch _yaw) (Math|Rotator|BreakRotator _returnvalue))
  (Transformation|SetActorRotation (Math|Rotator|MakeRotator (+ _roll 1e+01) _pitch _yaw) true))

(fn ConstructionScript)
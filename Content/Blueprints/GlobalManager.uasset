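; GlobalManager is an actor that tracks possession and supply counts and scatters Supply pickups around the player.
; On BeginPlay it binds a possession counter to the Inertial_PlayerController's PerformPossess event and sets a non-looping two-second timer.
; The timer spawns a batch of supplies at random positions around the player controller's location, at fixed height.
; Each supply's collect event increments the supply count and raises the possession limit by a refill amount.
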(event Custom|IncrementNumPossession
  (Variables|Default|SetnumPossession (+ (Variables|Default|GetnumPossession) 1)))

(event Custom|EventSpawnSupply
  (bind _returnvalue (Game|GetPlayerController 0))
  (bind _returnvalue_2 (Transformation|GetActorLocation _returnvalue))
  (bind (_x _y) (Math|Vector|BreakVector _returnvalue_2))
  (for _index (range 0 (Variables|Default|GetsupplySpawn))
    (bind _returnvalue_3 (Game|SpawnActorfromClass "/Game/Blueprints/Supply.Supply_C" (Math|Transform|MakeTransform (Math|Vector|MakeVector (Math|Random|RandomFloatinRange (- _x 1e+03) (+ _x 1e+03)) (Math|Random|RandomFloatinRange (- _y 1e+03) (+ _y 1e+03)) 2e+02)) "Undefined" 0 0))
    (EventDispatchers|BindEventtoCollectSupply _returnvalue_3 (delegate Custom|IncrementSupply))))

(event Custom|IncrementSupply
  (Variables|Default|SetnumSupply (+ (Variables|Default|GetnumSupply) 1))
  (Variables|Default|SetmaxPossession (+ (Variables|Default|GetmaxPossession) (Variables|Default|GetpossessRefill))))

(event EventBeginPlay
  (bind _asinertial_player_controller (Utilities|Casting|CastToInertial_PlayerController (Game|GetPlayerController 0)))
  (EventDispatchers|BindEventtoPerformPossess _asinertial_player_controller (delegate Custom|IncrementNumPossession))
  (Utilities|Time|SetTimerbyEvent (delegate Custom|EventSpawnSupply) 2.0))

(event Collision|EventActorBeginOverlap
  (params (OtherActor :type Actor%20Object%20Reference)))

(event EventTick
  (params (DeltaSeconds :type Float%20%28single-precision%29)))

(fn ConstructionScript)
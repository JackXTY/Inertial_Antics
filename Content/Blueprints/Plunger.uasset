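; Player-controllable plunger that walks with its box physics switched off, lifting slightly when control starts and leaving mouse actions empty.
; Walk does a swept move and, when blocked, traces forward low on the box to climb slopes under 70 degrees by realigning to the surface normal, or nudges up and forward if the trace misses.
; A bottom-contact helper traces to the base center and four corners, while CheckGround defers to the parent.
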(event EventBeginPlay
  (|CallParentFunction) ; This node is disabled and will not be called.\nDrag off pins to build functionality.
)

(event Collision|EventActorBeginOverlap
  (params (OtherActor :type Actor%20Object%20Reference))
  (|CallParentFunction OtherActor) ; This node is disabled and will not be called.\nDrag off pins to build functionality.
)

(event EventTick
  (params (DeltaSeconds :type Float%20%28single-precision%29))
  (|CallParentFunction DeltaSeconds) ; This node is disabled and will not be called.\nDrag off pins to build functionality.
)

(event EventOnMousePress)

(event EventOnMouseRelease
  (params (val :type Float%20%28single-precision%29)))

(event EventOnMousePressing
  (params (val :type Float%20%28single-precision%29)))

(event EventStartPlayerControl
  (Development|PrintString "plunger begin")
  (Variables|Default|SetStopingPlayer false)
  (Physics|SetSimulatePhysics (Variables|Default|GetBox) false)
  (Transformation|SetActorLocation (+ (Transformation|GetActorLocation) "0,0,10.000000") false false)
  (Variables|Default|SetOnGround true))

(fn ConstructionScript
  (|CallParentFunction))

(fn CheckGround
  (params (Time :type Float%20%28double-precision%29))
  (|CallParentFunction Time))

(fn Walk
  (params (time :type Float%20%28double-precision%29))
  (bind _returnvalue (Transformation|GetActorLocation))
  (bind _box (Variables|Default|GetBox))
  (bind _box_2 (Variables|Default|GetBox))
  (bind _box_3 (Variables|Default|GetBox))
  (bind _returnvalue_2 (Components|Box|GetScaledBoxExtent _box))
  (bind _returnvalue_3 (Components|Box|GetUnscaledBoxExtent _box_2))
  (bind (_x _y _z) (Math|Vector|BreakVector _returnvalue_2))
  (bind (_x_2 _y_2 _z_2) (Class|KismetMathLibrary|BreakVector3f _returnvalue_3))
  (bind _returnvalue_4 (- _z_2 15.0))
  (bind _returnvalue_5 (* _returnvalue_4 -1.0))
  (bind _returnvalue_6 (Math|Vector|MakeVector 0.0 0.0 _returnvalue_5))
  (bind _returnvalue_7 (+ _returnvalue _returnvalue_6))
  (Variables|Default|SetTime time)
  (bind _returnvalue_8 (Class|InertialPawn|GetWalkDirection))
  (LocalVariables|SetWalkDir _returnvalue_8)
  (if (> (Math|Vector|VectorLength _returnvalue_8) 0.5)
    (if (Class|SceneComponent|IsAnySimulatingPhysics _box_3)
      (Physics|SetSimulatePhysics _box_3 false)
      (Development|PrintString "Still simulating"))
    (bind _returnvalue_9 (Transformation|SetActorLocation (+ (* _returnvalue_8 (* time (Variables|Default|GetwalkPower))) (Transformation|GetActorLocation)) true false))
    (if (not _returnvalue_9)
      (bind (_outhit _returnvalue_10) (Collision|LineTraceByChannel _returnvalue_7 (+ _returnvalue_7 (* (LocalVariables|GetWalkDir) (+ _x_2 5e+01))) "TraceTypeQuery1" false 0 "ForDuration"))
      (if _returnvalue_10
        (bind _needtoclimb (CallFunction|CheckSlope (.ImpactNormal (Collision|BreakHitResult _outhit))))
        (if _needtoclimb
          (Development|PrintString "plunger climb Slope")
          (bind _result (CallFunction|BuildNewRotator (.ImpactNormal (Collision|BreakHitResult _outhit))))
          (bind _returnvalue_11 (Transformation|SetActorLocationAndRotation (+ (* (Math|Vector|RotateVector (Math|Vector|MakeVector (+ _x 1.0) 0.0 (+ _z 0.2)) _result) (* (* (Variables|Default|GetTime) (Variables|Default|GetwalkPower)) 0.3)) (.ImpactPoint (Collision|BreakHitResult _outhit))) _result true))
          (if _returnvalue_11
            _))
        (else
          (Transformation|SetActorLocation (+ (+ (Transformation|GetActorLocation) (* (LocalVariables|GetWalkDir) 3.0)) "0,0,3.000000") false false)
          (Development|PrintString "plunger climb UP!"))))))

(fn CheckifTouchBottom
  (bind _returnvalue (Transformation|GetActorLocation))
  (bind _returnvalue_2 (Transformation|GetActorLocation))
  (bind _box (Variables|Default|GetBox))
  (bind _returnvalue_3 (Components|Box|GetScaledBoxExtent _box))
  (bind (_x _y _z) (Class|KismetMathLibrary|BreakVector3f _returnvalue_3))
  (bind _returnvalue_4 (Collision|LineTraceByChannel _returnvalue_2 (+ _returnvalue_2 (* (Transformation|GetActorUpVector) (* (+ (.Z (Class|KismetMathLibrary|BreakVector3f (Components|Box|GetScaledBoxExtent (Variables|Default|GetBox)))) 1.0) -1.0))) "TraceTypeQuery1" false 0 "None"))
  (if _returnvalue_4
    (return true)
    (else
      (for _index (range 0 3)
        (bind _returnvalue_5 (Collision|LineTraceByChannel _returnvalue (+ _returnvalue (Math|Vector|MakeVector (* (Math|Float|SelectFloat -1.0 1.0 (< _index 2)) (- _x 0.5)) (* (Math|Float|SelectFloat -1.0 1.0 (== (Math|Integer|%(Integer) _index 2) 0)) (- _y 0.5)) (* (+ _z 1.0) -1.0))) "TraceTypeQuery1" false 0 "None"))
        (if _returnvalue_5
          (return true)))
      (return false))))

(fn BuildNewRotator
  (params (NewUp :type Vector))
  (bind _returnvalue (Transformation|GetActorForwardVector))
  (bind _returnvalue_2 (Math|Vector|CrossProduct NewUp _returnvalue))
  (return (Math|Rotator|MakeRotationfromAxes (Math|Vector|CrossProduct _returnvalue_2 NewUp) _returnvalue_2 NewUp)))

(fn CheckSlope
  (params (SlopeNormal :type Vector))
  (return (< (Class|KismetMathLibrary|DegAcos (Math|Vector|DotProduct SlopeNormal (Transformation|GetActorUpVector))) 7e+01)))